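; TrampomonsterBP is a single-use trampoline monster that bounces the SideScrollerCharacter upward.
; A swept overlap with its Box compares the character's Pound value to a threshold and picks one of three vertical launch strengths, overriding existing velocity.
; It then calls Slim and StopSliming on the character and clears ActionOccur.
; Any end overlap stops the stored character's jump and destroys the actor.
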(event `self.Box.OnComponentBeginOverlap`
  (params (OtherActor :type "Actor Object Reference") (OtherComp :type "PrimitiveComponent Object Reference") (OtherBodyIndex :type Integer) (bFromSweep :type Boolean) (SweepResult :type "HitResult Structure (by ref)"))
  (bind _character (`self.Character`))
  ;[1 1 1] TrampoJump
  (if bFromSweep
    (bind _asside_scroller_character (cast `/Game/SideScrollerBP/Blueprints/SideScrollerCharacter` OtherActor))
    (set `self.Character` _asside_scroller_character)
    (`/Engine/EditorBlueprintResources/StandardMacros.CompareFloat` (`/Game/SideScrollerBP/Blueprints/SideScrollerCharacter.Pound` (`self.Character`)) 0.5
      (:`>`
        (bind _output_get (set `self.JumpVelocity` (0.0 0.0 2000.0)))
        (`Character.LaunchCharacter` _character _output_get true true))
      (:`==`
        (bind _output_get_2 (set `self.JumpVelocity` (0.0 0.0 1500.0)))
        (`Character.LaunchCharacter` _character _output_get_2 true true))
      (:`<`
        (bind _output_get_3 (set `self.JumpVelocity` (0.0 0.0 1000.0)))
        (`Character.LaunchCharacter` _character _output_get_3 true true)))
    (`/Game/SideScrollerBP/Blueprints/SideScrollerCharacter.Slim` _character)
    (`/Game/SideScrollerBP/Blueprints/SideScrollerCharacter.Stop Sliming` _character)
    (set `/Game/SideScrollerBP/Blueprints/SideScrollerCharacter.actionOccur` false _character)))

(event `self.Box.OnComponentEndOverlap`
  (params (OtherActor :type "Actor Object Reference") (OtherComp :type "PrimitiveComponent Object Reference") (OtherBodyIndex :type Integer))
  ;[1 1 1] TrampoJump
  (`Character.StopJumping` (`self.Character`))
  (`self.K2_DestroyActor`))

(fn `UserConstructionScript`)